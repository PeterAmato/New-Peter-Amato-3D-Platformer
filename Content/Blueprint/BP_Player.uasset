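; BP_Player is a player-controlled Blueprint with Enhanced Input movement and jumping that reacts to hitting a goal object.
; IA_Move turns the controller yaw with X and moves along the yaw-only forward vector with Y, scaling both by RotationSpeed.
; IA_Jump triggers Jump on Started.
; A hit on a BP_GoalObject switches the Cube's material to BP_Orange.
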(event `self.ReceiveBeginPlay`)

(event `EnhancedInput|/Game/InputActions/IA_Move`
  (params (ActionValue :type "Vector2D Structure") (ElapsedSeconds :type "Float (double-precision)") (TriggeredSeconds :type "Float (double-precision)") (InputAction :type "InputAction Object Reference" :default "/Game/InputActions/IA_Move.IA_Move"))
  (bind (_x _y) (`KismetMathLibrary.BreakVector2D` ActionValue))
  (:`Triggered`
    (`self.AddControllerYawInput` (* _x (`self.RotationSpeed`)))
    (`self.AddMovementInput` (`KismetMathLibrary.GetForwardVector` (`KismetMathLibrary.MakeRotator` 0.0 0.0 (.yaw (`self.GetControlRotation`)))) (* _y (`self.RotationSpeed`)))))

(event `EnhancedInput|/Game/InputActions/IA_Jump`
  (params (ActionValue :type Boolean) (ElapsedSeconds :type "Float (double-precision)") (TriggeredSeconds :type "Float (double-precision)") (InputAction :type "InputAction Object Reference" :default "/Game/InputActions/IA_Jump.IA_Jump"))
  (:`Started`
    (`self.Jump`)))

(event `self.ReceiveHit`
  (params (MyComp :type "PrimitiveComponent Object Reference") (Other :type "Actor Object Reference") (OtherComp :type "PrimitiveComponent Object Reference") (bSelfMoved :type Boolean) (HitLocation :type "Vector Structure") (HitNormal :type "Vector Structure") (NormalImpulse :type "Vector Structure") (Hit :type "HitResult Structure (by ref)"))
  (cast `/Game/Levels/BP_GoalObject` Other)
  (`PrimitiveComponent.SetMaterial` (`self.Cube`) 0 "/Game/Materials/BP_Orange.BP_Orange"))

(fn `UserConstructionScript`)